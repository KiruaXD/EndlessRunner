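; Magnet power-up pickup for the endless runner that switches on the player's magnet for a few seconds.
; On player overlap it plays a sound, hides itself and, if no magnet is active, sets the player flag and game mode timer.
; A delayed loop counts the timer down each second while a separate Delay clears the flag and destroys the actor.
; It also destroys itself when overlapping an obstacle.
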(event `self.ReceiveActorBeginOverlap`
  (params (OtherActor :type "Actor Object Reference"))
  (`|ExecutionSequence`
    (:`then_0`
      (bind _asbp_player_character (cast `/Game/EndlessRunner/Blueprints/BP_PlayerCharacter_Quinn` OtherActor))
      (bind _asbp_runner_game_mode (cast `/Game/EndlessRunner/Blueprints/BP_RunnerGameMode` (`GameplayStatics.GetGameMode`)))
      (`GameplayStatics.PlaySound2D` "/Game/EndlessRunner/Meshes/350874__cabled_mess__coin_c_08.350874__cabled_mess__coin_c_08" 1.0 1.0 0.0 null null)
      (`self.SetActorHiddenInGame` true)
      (if (not (`/Game/EndlessRunner/Blueprints/BP_PlayerCharacter_Quinn.IsMagnetActive` _asbp_player_character))
        (set `/Game/EndlessRunner/Blueprints/BP_PlayerCharacter_Quinn.IsMagnetActive` true _asbp_player_character)
        (set `/Game/EndlessRunner/Blueprints/BP_RunnerGameMode.MagnetTimer` 6.0 _asbp_runner_game_mode)
        (`KismetSystemLibrary.PrintString` "Magnet Active")
        (`|ExecutionSequence`
          (:`then_0`
            (`/Game/EndlessRunner/Blueprints/Inputs/ForLoopDelay.ForLoopWithDelay` 0 5 1.0
              (:`LoopBody`
                (bind _result (`/Engine/EditorBlueprintResources/StandardMacros.DecrementFloat` (`/Game/EndlessRunner/Blueprints/BP_RunnerGameMode.MagnetTimer` _asbp_runner_game_mode))
                  (:`  `
                    (bind _output_get (set `/Game/EndlessRunner/Blueprints/BP_RunnerGameMode.MagnetTimer` (`KismetMathLibrary.FMax` _result) _asbp_runner_game_mode))
                    (`KismetSystemLibrary.PrintString` (`KismetStringLibrary.Conv_DoubleToString` _output_get) true true (struct :`R` 0.908402 :`G` 1.0 :`B` 0.299821 :`A` 1.0)))))))
          (:`then_1`
            (`KismetSystemLibrary.Delay` 5.2)
            (bind _asbp_player_character_2 (cast `/Game/EndlessRunner/Blueprints/BP_PlayerCharacter_Quinn` (`GameplayStatics.GetPlayerCharacter` 0)))
            (set `/Game/EndlessRunner/Blueprints/BP_PlayerCharacter_Quinn.IsMagnetActive` false _asbp_player_character_2)
            (`KismetSystemLibrary.PrintString` "Magnet InActive")
            (`self.K2_DestroyActor`)))))
    (:`then_1`
      (cast `/Game/EndlessRunner/Blueprints/Obstacles/BP_Obstacles` OtherActor)
      (`self.K2_DestroyActor`))))

(fn `UserConstructionScript`)