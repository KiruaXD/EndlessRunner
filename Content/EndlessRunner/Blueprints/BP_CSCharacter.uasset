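; Character-selection Blueprint for the endless runner that previews Manny or Quinn and commits the player's choice.
; Show events toggle which of the two previews is visible, while Spawn events pass the matching player character as a Pawn to SaveCharacter rather than spawning it.
; SaveCharacter loads or creates the Runner_SaveGame in the PlayerCharacter slot, stores the choice, then opens Runner_Map.
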(event `Show Quinn`
  (`SceneComponent.SetHiddenInGame` (`self.Quinn`) false false)
  (`SceneComponent.SetHiddenInGame` (`self.Manny`) true false))

(event `Show Manny`
  (`SceneComponent.SetHiddenInGame` (`self.Manny`) false false)
  (`SceneComponent.SetHiddenInGame` (`self.Quinn`) true false))

(event `Spawn Quinn`
  (bind _aspawn (castclass `Pawn` "/Game/EndlessRunner/Blueprints/BP_PlayerCharacter_Quinn.BP_PlayerCharacter_Quinn_C"))
  (bind _output_get (set `self.As Pawn` _aspawn))
  (`self.SaveCharacter` _output_get))

(event `Spawn Manny`
  (bind _aspawn (castclass `Pawn` "/Game/EndlessRunner/Blueprints/BP_PlayerCharacter_Manny1.BP_PlayerCharacter_Manny1_C"))
  (bind _output_get (set `self.As Pawn` _aspawn))
  (`self.SaveCharacter` _output_get))

(fn `SaveCharacter`
  (params (PlayerCharacter :type "Pawn Class Reference"))
  (bind _returnvalue (`GameplayStatics.DoesSaveGameExist` "PlayerCharacter"))
  (if _returnvalue
    (bind _returnvalue_2 (`GameplayStatics.LoadGameFromSlot` "PlayerCharacter"))
    (bind _output_get (set `self.Saver Sub Class` _returnvalue_2))
    (bind _asrunner_save_game (cast `/Game/EndlessRunner/Blueprints/Runner_SaveGame` _output_get))
    (set `/Game/EndlessRunner/Blueprints/Runner_SaveGame.PlayerCharacter` PlayerCharacter _asrunner_save_game)
    (`GameplayStatics.SaveGameToSlot` (`self.Saver Sub Class`) "PlayerCharacter")
    (else
      (bind _returnvalue_3 (`GameplayStatics.CreateSaveGameObject` "/Game/EndlessRunner/Blueprints/Runner_SaveGame.Runner_SaveGame_C"))
      (bind _output_get_2 (set `self.Saver Sub Class` _returnvalue_3))
      (bind _asrunner_save_game_2 (cast `/Game/EndlessRunner/Blueprints/Runner_SaveGame` _output_get_2))
      (set `/Game/EndlessRunner/Blueprints/Runner_SaveGame.PlayerCharacter` PlayerCharacter _asrunner_save_game_2)
      (`GameplayStatics.SaveGameToSlot` (`self.Saver Sub Class`) "PlayerCharacter")))
  (`GameplayStatics.OpenLevelBySoftObjectPtr` "/Game/EndlessRunner/Maps/Runner_Map.Runner_Map"))

(fn `UserConstructionScript`)