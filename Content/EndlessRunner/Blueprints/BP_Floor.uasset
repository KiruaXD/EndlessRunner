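; Endless runner floor tile that fills itself with random obstacles, coins and power-ups and exposes an arrow transform as its attach point.
; The construction script builds per-lane arrow grids, shuffles their transforms and spawns child actors, with game mode floor counters gating power-ups and cars.
; Box overlap asks BP_RunnerGameMode to extend the floor, slightly raises the player's clamped walk speed and adds multiplier-scaled points.
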(event `self.Box.OnComponentBeginOverlap`
  (params (OverlappedComponent :type "PrimitiveComponent Object Reference") (OtherActor :type "Actor Object Reference") (OtherComp :type "PrimitiveComponent Object Reference") (OtherBodyIndex :type Integer) (bFromSweep :type Boolean) (SweepResult :type "HitResult Structure (by ref)"))
  ;[0.02127 0.1246 0.15] Extend Floor
  (bind _asbp_runner_game_mode (cast `/Game/EndlessRunner/Blueprints/BP_RunnerGameMode` (`GameplayStatics.GetGameMode`)))
  (`/Game/EndlessRunner/Blueprints/BP_RunnerGameMode.Extend Floor` _asbp_runner_game_mode)
  ;[0.15 0.02352 0.01865] Change Speed
  (bind _asbp_player_character_quinn (cast `/Game/EndlessRunner/Blueprints/BP_PlayerCharacter_Quinn` (`GameplayStatics.GetPlayerCharacter` 0)))
  (bind _charactermovement (`Character.CharacterMovement` _asbp_player_character_quinn))
  (bind _output_get (set `CharacterMovementComponent.MaxWalkSpeed` (`KismetMathLibrary.FClamp` (* (`CharacterMovementComponent.MaxWalkSpeed` _charactermovement) 1.001) 700.0 1500.0) _charactermovement))
  (`KismetSystemLibrary.PrintString` (`KismetStringLibrary.Conv_DoubleToString` _output_get))
  ;[0.15 0.1451 0.007059] Set Points
  (bind _asbp_runner_game_mode_2 (cast `/Game/EndlessRunner/Blueprints/BP_RunnerGameMode` (`GameplayStatics.GetGameMode`)))
  (set `/Game/EndlessRunner/Blueprints/BP_RunnerGameMode.CurrentPoints` (+ (* (`/Game/EndlessRunner/Blueprints/BP_RunnerGameMode.PointsMulti` _asbp_runner_game_mode_2) 1) (`/Game/EndlessRunner/Blueprints/BP_RunnerGameMode.CurrentPoints` _asbp_runner_game_mode_2)) _asbp_runner_game_mode_2))

(fn `CoinSpawnPoints`
  (for _array_element (`self.LanePostion`)
    (for _index (range 10)
      (bind _returnvalue (`AddComponent|NODE_AddArrowComponent-3` :`RelativeTransform` (`KismetMathLibrary.MakeTransform` (`KismetMathLibrary.MakeVector` (* _index 75.0) _array_element))))
      (`ArrowComponent.SetArrowColor` _returnvalue (struct :`B` 1.0 :`A` 1.0))
      (`KismetArrayLibrary.Array_Add` (`self.CSpawnPoints`) (`SceneComponent.K2_GetComponentToWorld` _returnvalue)))))

(fn `GetAttachPoint`
  (returns (ReturnValue :type "Transform Structure"))
  (return (`SceneComponent.K2_GetComponentToWorld` (`self.Arrow`))))

(fn `PowerUpSpawnPoints`
  (for _array_element (`self.LanePostion`)
    (for _index (range 3)
      (bind _returnvalue (`AddComponent|NODE_AddArrowComponent-4` :`RelativeTransform` (`KismetMathLibrary.MakeTransform` (`KismetMathLibrary.MakeVector` (* _index 250.0) _array_element))))
      (`ArrowComponent.SetArrowColor` _returnvalue (struct :`G` 1.0 :`A` 1.0))
      (`KismetArrayLibrary.Array_Add` (`self.PSpawnPoints`) (`SceneComponent.K2_GetComponentToWorld` _returnvalue)))))

(fn `SetupSpawnPoints`
  (for _array_element (`self.LanePostion`)
    (for _index (range 2)
      (bind _returnvalue (`AddComponent|NODE_AddArrowComponent-0` :`RelativeTransform` (`KismetMathLibrary.MakeTransform` (`KismetMathLibrary.MakeVector` (* _index 650.0) _array_element))))
      (`KismetArrayLibrary.Array_Add` (`self.SpawnPoints`) (`SceneComponent.K2_GetComponentToWorld` _returnvalue)))))

(fn `SpawnCars`
  (params (Selection :type Integer) (RelativeTransform :type "Transform Structure"))
  (bind _asbp_runner_game_mode (cast `/Game/EndlessRunner/Blueprints/BP_RunnerGameMode` (`GameplayStatics.GetGameMode`)))
  (if (> (`/Game/EndlessRunner/Blueprints/BP_RunnerGameMode.FloorCountForMovingObstacles` _asbp_runner_game_mode) (`KismetMathLibrary.RandomIntegerInRange` 5 10))
    (switch `int` Selection
      (:`Default`
        _)
      (:`0`
        _)
      (:`1`
        _))
    (`AddComponent|NODE_AddChildActorComponent-6` :`RelativeTransform` RelativeTransform)
    (set `/Game/EndlessRunner/Blueprints/BP_RunnerGameMode.FloorCountForMovingObstacles` 0 _asbp_runner_game_mode)))

(fn `SpawnCoins`
  (locals (RandomSpawnPoints :type "Array of Transform Structure"))
  (bind _output_get (set `local.RandomSpawnPoints` (`self.CSpawnPoints`)))
  (`KismetArrayLibrary.Array_Shuffle` _output_get)
  (for _index (range (+ (`KismetMathLibrary.RandomIntegerInRange` 5 8) 1))
    (`AddComponent|NODE_AddChildActorComponent-4` :`RelativeTransform` (`KismetMathLibrary.MakeRelativeTransform` (`|GetArrayItem` (`local.RandomSpawnPoints`) _index) (`self.GetTransform`)))))

(fn `SpawnObstacles`
  (locals (RandomSpawnPoints :type "Array of Transform Structure"))
  (bind _output_get (set `local.RandomSpawnPoints` (`self.SpawnPoints`)))
  (`KismetArrayLibrary.Array_Shuffle` _output_get)
  (for _index (range (+ (`KismetMathLibrary.RandomIntegerInRange` 0 1) 1))
    (switch `int` (`KismetMathLibrary.RandomIntegerInRange` 0 3)
      (:`0`
        (bind _returnvalue (`KismetMathLibrary.MakeRelativeTransform` (`|GetArrayItem` (`local.RandomSpawnPoints`) _index) (`self.GetTransform`)))
        (`AddComponent|NODE_AddChildActorComponent-0` :`RelativeTransform` _returnvalue))
      (:`1`
        (`AddComponent|NODE_AddChildActorComponent-1` :`RelativeTransform` _returnvalue))
      (:`2`
        (`self.SpawnCars` 0 _returnvalue :!label _label))
      (:`3`
        (goto _label)))))

(fn `SpawnPowerUps`
  (locals (RandomSpawnPoints :type "Array of Transform Structure"))
  (bind _returnvalue (`KismetMathLibrary.MakeRelativeTransform` (`|GetArrayItem` (`local.RandomSpawnPoints`)) (`self.GetTransform`)))
  (bind _asbp_runner_game_mode (cast `/Game/EndlessRunner/Blueprints/BP_RunnerGameMode` (`GameplayStatics.GetGameMode`)))
  (if (> (`/Game/EndlessRunner/Blueprints/BP_RunnerGameMode.FloorCount` _asbp_runner_game_mode) 5)
    (bind _output_get (set `local.RandomSpawnPoints` (`self.PSpawnPoints`)))
    (`KismetArrayLibrary.Array_Shuffle` _output_get)
    (switch `int` (`KismetMathLibrary.RandomIntegerInRange` 0 1)
      (:`0`
        (`AddComponent|NODE_AddChildActorComponent-5` :`RelativeTransform` _returnvalue))
      (:`1`
        (`AddComponent|NODE_AddChildActorComponent-7` :`RelativeTransform` _returnvalue)))
    (set `/Game/EndlessRunner/Blueprints/BP_RunnerGameMode.FloorCount` 0 _asbp_runner_game_mode)))

(fn `UserConstructionScript`
  (`self.SetupSpawnPoints`)
  (`self.SpawnObstacles`)
  (`self.CoinSpawnPoints`)
  (`self.SpawnCoins`)
  (`self.PowerUpSpawnPoints`)
  (`self.SpawnPowerUps`))