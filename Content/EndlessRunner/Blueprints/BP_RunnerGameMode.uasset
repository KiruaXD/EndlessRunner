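; Endless runner game mode that builds and recycles the track and roadside buildings and loads saved coins.
; BeginPlay spawns initial floor tiles and buildings, reading Coins from the CoinValue save slot inside the floor loop.
; Each piece spawns at the previous one's attach point, with floor spawns also incrementing counters, including one for moving obstacles.
; ExtendFloor and ExtendBuildings append a piece and destroy the oldest once their array exceeds its limit.
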(event `self.ReceiveBeginPlay`
  (`|ExecutionSequence`
    (:`then_0`
      (for _ (range (`self.Number of Tiles`))
        (`self.Add Floor`)
        (bind _returnvalue (`GameplayStatics.LoadGameFromSlot` "CoinValue"))
        (bind _asrunner_save_game (cast `/Game/EndlessRunner/Blueprints/Runner_SaveGame` _returnvalue))
        (set `self.Coins` (`/Game/EndlessRunner/Blueprints/Runner_SaveGame.CoinValue` _asrunner_save_game))))
    (:`then_1`
      (for _ (range 6)
        (`self.AddBuildings`)))))

(fn `Add Floor`
  (bind _returnvalue (`|SpawnActorFromClass` "/Game/EndlessRunner/Blueprints/BP_Floor.BP_Floor_C" (`self.Floor Attach Point`) "Undefined" "MultiplyWithRoot" null null))
  (bind _returnvalue_2 (`/Game/EndlessRunner/Blueprints/BP_Floor.GetAttachPoint` _returnvalue))
  (set `self.Floor Attach Point` _returnvalue_2)
  (`KismetArrayLibrary.Array_Add` (`self.Floor Tiles`) _returnvalue)
  (bind _result (`/Engine/EditorBlueprintResources/StandardMacros.IncrementInt` (`self.FloorCount`))
    (:`  `
      (set `self.FloorCount` _result)
      (bind _result_2 (`/Engine/EditorBlueprintResources/StandardMacros.IncrementInt` (`self.FloorCountForMovingObstacles`))
        (:`  `
          (set `self.FloorCountForMovingObstacles` _result_2))))))

(fn `AddBuildings`
  (bind _returnvalue (`|SpawnActorFromClass` "/Game/EndlessRunner/Blueprints/BP_Buildings.BP_Buildings_C" (`self.Building Spawn Point`) "Undefined" "MultiplyWithRoot" null null))
  (bind _returnvalue_2 (`/Game/EndlessRunner/Blueprints/BP_Buildings.GetAttachPoint` _returnvalue))
  (set `self.Building Spawn Point` _returnvalue_2)
  (`KismetArrayLibrary.Array_Add` (`self.BP_BuildingsArr`) _returnvalue))

(fn `Extend Floor`
  (bind _floor_tiles (`self.Floor Tiles`))
  (bind _output (`|GetArrayItem` _floor_tiles))
  (`self.Add Floor`)
  (if (> (`KismetArrayLibrary.Array_Length` (`self.Floor Tiles`)) (+ (`self.Number of Tiles`) 10))
    (`self.K2_DestroyActor` _output)
    (`KismetArrayLibrary.Array_RemoveItem` _floor_tiles _output)))

(fn `ExtendBuildings`
  (bind _bp_buildingsarr (`self.BP_BuildingsArr`))
  (bind _output (`|GetArrayItem` _bp_buildingsarr))
  (`self.AddBuildings`)
  (if (> (`KismetArrayLibrary.Array_Length` (`self.BP_BuildingsArr`)) 4)
    (`self.K2_DestroyActor` _output)
    (`KismetArrayLibrary.Array_RemoveItem` _bp_buildingsarr _output)))

(fn `UserConstructionScript`)