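; BP_Buildings is a tile of roadside buildings for an endless runner that grows the scenery as play progresses.
; Its construction script adds random meshes from BuildingList at six spawn-point components, turning one set of three 180 degrees in yaw.
; Overlapping its Box tells BP_RunnerGameMode to extend the buildings.
; GetAttachPoint returns the Arrow transform pushed far along world X as an attach point.
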(event `self.Box.OnComponentBeginOverlap`
  (params (OverlappedComponent :type "PrimitiveComponent Object Reference") (OtherActor :type "Actor Object Reference") (OtherComp :type "PrimitiveComponent Object Reference") (OtherBodyIndex :type Integer) (bFromSweep :type Boolean) (SweepResult :type "HitResult Structure (by ref)"))
  ;[0.02127 0.1246 0.15] Extend Floor
  (bind _asbp_runner_game_mode (cast `/Game/EndlessRunner/Blueprints/BP_RunnerGameMode` (`GameplayStatics.GetGameMode`)))
  (`/Game/EndlessRunner/Blueprints/BP_RunnerGameMode.ExtendBuildings` _asbp_runner_game_mode))

(fn `GetAttachPoint`
  (returns (ReturnValue :type "Transform Structure"))
  (return (`KismetMathLibrary.MakeTransform` (`KismetMathLibrary.MakeVector` (+ (.x (.location (`SceneComponent.K2_GetComponentToWorld` (`self.Arrow`)))) 13000.0) (.y (.location (`SceneComponent.K2_GetComponentToWorld` (`self.Arrow`)))) (.z (.location (`SceneComponent.K2_GetComponentToWorld` (`self.Arrow`))))) (.rotation (`SceneComponent.K2_GetComponentToWorld` (`self.Arrow`))) (.scale (`SceneComponent.K2_GetComponentToWorld` (`self.Arrow`))))))

(fn `RandomBuildingSpawner`
  (returns (OutItem :type "StaticMesh Object Reference"))
  (locals (BuildingList :type "Array of StaticMesh Object Reference"))
  (return (`KismetArrayLibrary.Array_Random` (`local.BuildingList`))))

(fn `SpawnBuildings`
  (`|ExecutionSequence`
    (:`then_0`
      (for _array_element (`|MakeArray` (`self.Sp1`) (`self.Sp3`) (`self.Sp4`))
        (bind _returnvalue (`AddComponent|NODE_AddStaticMeshComponent-0` :`RelativeTransform` (`SceneComponent.GetRelativeTransform` _array_element)))
        (bind _outitem (`self.RandomBuildingSpawner`))
        (`StaticMeshComponent.SetStaticMesh` _returnvalue _outitem)))
    (:`then_1`
      (for _array_element_2 (`|MakeArray` (`self.Sp2`) (`self.Sp5`) (`self.Sp6`))
        (bind _returnvalue_2 (`AddComponent|NODE_AddStaticMeshComponent-1` :`RelativeTransform` (`KismetMathLibrary.MakeTransform` (.location (`SceneComponent.GetRelativeTransform` _array_element_2)) (`KismetMathLibrary.MakeRotator` (.roll (.rotation (`SceneComponent.GetRelativeTransform` _array_element_2))) (.pitch (.rotation (`SceneComponent.GetRelativeTransform` _array_element_2))) (+ (.yaw (.rotation (`SceneComponent.GetRelativeTransform` _array_element_2))) 180.0)) (.scale (`SceneComponent.GetRelativeTransform` _array_element_2)))))
        (bind _outitem_2 (`self.RandomBuildingSpawner`))
        (`StaticMeshComponent.SetStaticMesh` _returnvalue_2 _outitem_2)))))

(fn `UserConstructionScript`
  (`self.SpawnBuildings`))