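; BP_Obstacles_Blocker is an endless runner obstacle that kills the player on contact unless they are sliding.
; On actor overlap it casts the other actor to BP_PlayerCharacter_Quinn and checks its IsSliding flag.
; When the player is not sliding, it calls Death on the character, waits briefly, then pauses the game.
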(event `self.ReceiveActorBeginOverlap`
  (params (OtherActor :type "Actor Object Reference"))
  (bind _asbp_player_character (cast `/Game/EndlessRunner/Blueprints/BP_PlayerCharacter_Quinn` OtherActor))
  (if (not (`/Game/EndlessRunner/Blueprints/BP_PlayerCharacter_Quinn.IsSliding` _asbp_player_character))
    (`/Game/EndlessRunner/Blueprints/BP_PlayerCharacter_Quinn.Death` _asbp_player_character)
    (`KismetSystemLibrary.Delay` 1.0)
    (`GameplayStatics.SetGamePaused` true)))

(fn `UserConstructionScript`
  (`parent.UserConstructionScript`))