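; Collectible coin for the endless runner that adds to the game mode's coin count when the player touches it.
; Pickup prints the total, plays a sound, destroys the coin and calls the player's UpdateCoins.
; Coins overlapping obstacles destroy themselves.
; An outer sphere detects a player with an active magnet and starts a timeline that interpolates the coin toward the player, adding the track value as an offset.
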(event `self.Coin.OnComponentBeginOverlap`
  (params (OverlappedComponent :type "PrimitiveComponent Object Reference") (OtherActor :type "Actor Object Reference") (OtherComp :type "PrimitiveComponent Object Reference") (OtherBodyIndex :type Integer) (bFromSweep :type Boolean) (SweepResult :type "HitResult Structure (by ref)"))
  (`|ExecutionSequence`
    (:`then_0`
      (bind _asbp_player_character (cast `/Game/EndlessRunner/Blueprints/BP_PlayerCharacter_Quinn` OtherActor))
      (bind _asbp_runner_game_mode (cast `/Game/EndlessRunner/Blueprints/BP_RunnerGameMode` (`GameplayStatics.GetGameMode`)))
      (bind _coins (`/Game/EndlessRunner/Blueprints/BP_RunnerGameMode.Coins` _asbp_runner_game_mode))
      (`/Engine/EditorBlueprintResources/StandardMacros.IncrementInt` _coins
        (:`  `
          (`KismetSystemLibrary.PrintString` (`KismetStringLibrary.Conv_IntToString` _coins))
          (`GameplayStatics.PlaySound2D` "/Game/EndlessRunner/Meshes/350874__cabled_mess__coin_c_08.350874__cabled_mess__coin_c_08" 1.0 1.0 0.0 null null)
          (`self.K2_DestroyActor`)
          (`/Game/EndlessRunner/Blueprints/BP_PlayerCharacter_Quinn.UpdateCoins` _asbp_player_character))))
    (:`then_1`
      (cast `/Game/EndlessRunner/Blueprints/Obstacles/BP_Obstacles` OtherActor)
      (`self.K2_DestroyActor`))
    (:`then_2`
      (cast `/Game/EndlessRunner/Blueprints/BP_PlayerCharacter_Quinn` OtherActor)
      (`self.K2_DestroyActor`))))

(event `self.Sphere.OnComponentBeginOverlap`
  (params (OverlappedComponent :type "PrimitiveComponent Object Reference") (OtherActor :type "Actor Object Reference") (OtherComp :type "PrimitiveComponent Object Reference") (OtherBodyIndex :type Integer) (bFromSweep :type Boolean) (SweepResult :type "HitResult Structure (by ref)"))
  (bind _asbp_player_character (cast `/Game/EndlessRunner/Blueprints/BP_PlayerCharacter_Quinn` OtherActor))
  (if (`/Game/EndlessRunner/Blueprints/BP_PlayerCharacter_Quinn.IsMagnetActive` _asbp_player_character)
    (bind (_direction _track) (`Timeline|Timeline` :!via `PlayFromStart`)
      (:`Update`
        (`self.K2_SetActorLocation` (+ _track (`KismetMathLibrary.VInterpTo` (.location (`self.GetTransform`)) (`self.K2_GetActorLocation` (`GameplayStatics.GetPlayerCharacter` 0)) (`GameplayStatics.GetWorldDeltaSeconds`) 20.0)))))))

(fn `UserConstructionScript`)