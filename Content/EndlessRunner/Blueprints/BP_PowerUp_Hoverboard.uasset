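; Hoverboard power-up pickup for the endless runner that puts the player into a timed hover state.
; On player overlap it plays a sound, hides itself and, unless already hovering, shows the player's board and starts the game mode's HoverTimer.
; A delayed loop counts the timer down; hover ending early or a parallel Delay hides the board and destroys the pickup.
; Any BP_Obstacles actor overlapping the pickup is destroyed.
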(event `self.Hoverboard.OnComponentBeginOverlap`
  (params (OverlappedComponent :type "PrimitiveComponent Object Reference") (OtherActor :type "Actor Object Reference") (OtherComp :type "PrimitiveComponent Object Reference") (OtherBodyIndex :type Integer) (bFromSweep :type Boolean) (SweepResult :type "HitResult Structure (by ref)"))
  (`|ExecutionSequence`
    (:`then_0`
      (bind _asbp_player_character_quinn (cast `/Game/EndlessRunner/Blueprints/BP_PlayerCharacter_Quinn` OtherActor))
      (bind _asbp_runner_game_mode (cast `/Game/EndlessRunner/Blueprints/BP_RunnerGameMode` (`GameplayStatics.GetGameMode`)))
      (`GameplayStatics.PlaySound2D` "/Engine/VREditor/Sounds/UI/Camera_Shutter.Camera_Shutter" 1.0 1.0 0.0 null null)
      (`self.SetActorHiddenInGame` true)
      (if (not (`/Game/EndlessRunner/Blueprints/BP_PlayerCharacter_Quinn.IsHovering` _asbp_player_character_quinn))
        (set `/Game/EndlessRunner/Blueprints/BP_RunnerGameMode.HoverTimer` 10.0 _asbp_runner_game_mode)
        (set `/Game/EndlessRunner/Blueprints/BP_PlayerCharacter_Quinn.IsHovering` true _asbp_player_character_quinn)
        (`SceneComponent.SetHiddenInGame` (`/Game/EndlessRunner/Blueprints/BP_PlayerCharacter_Quinn.Hoverboard` _asbp_player_character_quinn) false false)
        (`KismetSystemLibrary.PrintString` "Hover Active")
        (`|ExecutionSequence`
          (:`then_0`
            (`/Game/EndlessRunner/Blueprints/Inputs/ForLoopDelay.ForLoopWithDelay` 0 10 1.0
              (:`LoopBody`
                (bind _asbp_player_character_quinn_2 (cast `/Game/EndlessRunner/Blueprints/BP_PlayerCharacter_Quinn` (`GameplayStatics.GetPlayerCharacter` 0)))
                (if (`/Game/EndlessRunner/Blueprints/BP_PlayerCharacter_Quinn.IsHovering` _asbp_player_character_quinn_2)
                  (bind _result (`/Engine/EditorBlueprintResources/StandardMacros.DecrementFloat` (`/Game/EndlessRunner/Blueprints/BP_RunnerGameMode.HoverTimer` _asbp_runner_game_mode))
                    (:`  `
                      (set `/Game/EndlessRunner/Blueprints/BP_RunnerGameMode.HoverTimer` (`KismetMathLibrary.FMax` _result) _asbp_runner_game_mode)))
                  (else
                    (bind _asbp_player_character_quinn_3 (cast `/Game/EndlessRunner/Blueprints/BP_PlayerCharacter_Quinn` (`GameplayStatics.GetPlayerCharacter` 0) :!label _label))
                    (set `/Game/EndlessRunner/Blueprints/BP_PlayerCharacter_Quinn.IsHovering` false _asbp_player_character_quinn_3)
                    (`SceneComponent.SetHiddenInGame` (`/Game/EndlessRunner/Blueprints/BP_PlayerCharacter_Quinn.Hoverboard` _asbp_player_character_quinn_3) true false)
                    (`self.K2_DestroyActor`))))))
          (:`then_1`
            (`KismetSystemLibrary.Delay` 10.2)
            (goto _label)))))
    (:`then_1`
      (bind _asbp_obstacles (cast `/Game/EndlessRunner/Blueprints/Obstacles/BP_Obstacles` OtherActor))
      (`self.K2_DestroyActor` _asbp_obstacles))))

(fn `UserConstructionScript`)