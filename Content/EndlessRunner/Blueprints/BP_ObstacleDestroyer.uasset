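; BP_ObstacleDestroyer is an endless runner actor that clears obstacles it overlaps while the player is dead or hovering.
; On overlap it reads those flags from the player character, then destroys the other actor if it is a Blocker or Wall obstacle and itself after a short delay.
; If the player is neither dead nor hovering, it destroys itself immediately on any overlap.
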(event `self.ReceiveActorBeginOverlap`
  (params (OtherActor :type "Actor Object Reference"))
  (bind _asbp_player_character_quinn (cast `/Game/EndlessRunner/Blueprints/BP_PlayerCharacter_Quinn` (`GameplayStatics.GetPlayerCharacter` 0)))
  (if (or (`/Game/EndlessRunner/Blueprints/BP_PlayerCharacter_Quinn.IsDead` _asbp_player_character_quinn) (`/Game/EndlessRunner/Blueprints/BP_PlayerCharacter_Quinn.IsHovering` _asbp_player_character_quinn))
    (`|ExecutionSequence`
      (:`then_0`
        (bind _asbp_obstacles_blocker (cast `/Game/EndlessRunner/Blueprints/Obstacles/BP_Obstacles_Blocker` OtherActor))
        (`self.K2_DestroyActor` _asbp_obstacles_blocker))
      (:`then_1`
        (bind _asbp_obstacles_wall (cast `/Game/EndlessRunner/Blueprints/Obstacles/BP_Obstacles_Wall` OtherActor))
        (`self.K2_DestroyActor` _asbp_obstacles_wall)))
    (`KismetSystemLibrary.Delay` 0.5)
    (`self.K2_DestroyActor`)
    (else
      (`self.K2_DestroyActor`))))

(fn `UserConstructionScript`)